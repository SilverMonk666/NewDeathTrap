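; Moving pole actor that travels a continuous closed loop from its start position through three endpoint components and back.
; On BeginPlay it caches those world locations, then four chained timelines lerp the pole along each leg with swept moves.
; Each timeline starts the next on finish, and the last calls MovePlatform to restart the loop.
; The PlayRate variable is applied to the first three timelines only, not the return leg.
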(event `self.ReceiveBeginPlay`
  (set `self.Startlocation` (`SceneComponent.K2_GetComponentLocation` (`self.NewPlaceholderPole`)))
  (set `self.EndPointLocation01` (`SceneComponent.K2_GetComponentLocation` (`self.Endpoint01`)))
  (set `self.EndPointLocation02` (`SceneComponent.K2_GetComponentLocation` (`self.EndPoint02`)))
  (set `self.EndPointLocation03` (`SceneComponent.K2_GetComponentLocation` (`self.EndPoint03`)))
  (`TimelineComponent.SetPlayRate` (`self.MovePlat`) (`self.PlayRate`))
  (`TimelineComponent.SetPlayRate` (`self.Timeline_0`) (`self.PlayRate`))
  (`TimelineComponent.SetPlayRate` (`self.Timeline_1`) (`self.PlayRate`))
  (bind (_direction _moveplat) (`Timeline|MovePlat` :`NewTime` (`self.NewTime`) :!label _label)
    (:`Update`
      (`SceneComponent.K2_SetWorldLocation` (`self.NewPlaceholderPole`) (`KismetMathLibrary.VLerp` (`self.Startlocation`) (`self.EndPointLocation01`) _moveplat) true false))
    (:`Finished`
      (bind (_direction_2 _moveplat_2) (`Timeline|Timeline_0` :`NewTime` (`self.NewTime`) :!via `PlayFromStart`)
        (:`Update`
          (`SceneComponent.K2_SetWorldLocation` (`self.NewPlaceholderPole`) (`KismetMathLibrary.VLerp` (`self.EndPointLocation01`) (`self.EndPointLocation02`) _moveplat_2) true false))
        (:`Finished`
          (bind (_direction_3 _moveplat_3) (`Timeline|Timeline_1` :`NewTime` (`self.NewTime`) :!via `PlayFromStart`)
            (:`Update`
              (`SceneComponent.K2_SetWorldLocation` (`self.NewPlaceholderPole`) (`KismetMathLibrary.VLerp` (`self.EndPointLocation02`) (`self.EndPointLocation03`) _moveplat_3) true false))
            (:`Finished`
              (bind (_direction_4 _moveplat_4) (`Timeline|Timeline_2` :`NewTime` (`self.NewTime`) :!via `PlayFromStart`)
                (:`Update`
                  (`SceneComponent.K2_SetWorldLocation` (`self.NewPlaceholderPole`) (`KismetMathLibrary.VLerp` (`self.EndPointLocation03`) (`self.Startlocation`) _moveplat_4) true false))
                (:`Finished`
                  (`self.MovePlatform`))))))))))

(event `MovePlatform`
  (goto _label :!via `PlayFromStart`))

(fn `UserConstructionScript`
  (`parent.UserConstructionScript`))