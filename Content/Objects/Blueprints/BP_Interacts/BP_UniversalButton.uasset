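; BP_UniversalButton is an interactable button that toggles an on/off state and pushes it to a list of target actors.
; Interact flips the two-value OnOffState enum, then calls Activate, which sends SwitchStateMessage with the new state to each entry in ActorsToEffect and prints it.
; BeginPlay sends the same message to sync targets with the initial state.
; The button's own SwitchState function is a stub returning false.
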(event `self.ReceiveBeginPlay`
  (for _array_element (`self.ActorsToEffect`)
    (message `/Game/Objects/BP_ButtonInterface.SwitchState` _array_element (`self.OnOffState`))))

(event `Activate`
  (bind _onoffstate (`self.OnOffState`))
  (for _array_element (`self.ActorsToEffect`)
    (message `/Game/Objects/BP_ButtonInterface.SwitchState` _array_element _onoffstate)
    (`KismetSystemLibrary.PrintString` (`|GetEnumeratorNameAsString` _onoffstate))))

(fn `Interact`
  (params (TargetPoint :type "SceneComponent Object Reference") (Actor :type "Actor Object Reference"))
  (returns (Val :type Boolean))
  (if (`|EnumEquality` (`self.OnOffState`) "NewEnumerator0")
    (set `self.OnOffState` "NewEnumerator1")
    (else
      (set `self.OnOffState` "NewEnumerator0")))
  (`self.Activate`)
  (return false))

(fn `SwitchState`
  (returns (NewParam :type Boolean) (NewParam :type Boolean))
  (return false false))

(fn `UserConstructionScript`)