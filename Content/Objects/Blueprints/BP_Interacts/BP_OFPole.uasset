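; BP_OFPole is an on/off pole that moves the player character to its Arrow's location on an action press.
; SwitchState stores the state and toggles particle visibility to match.
; Tick polls the player's action button and, while they overlap the Trigger and the pole is on, eases the capsule across with MoveComponentTo, stopping its movement.
; A DoOnce limits this to one move until the button is released.
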(event `self.ReceiveBeginPlay`
  (switch `/Game/Objects/Misc/E_OnOFfStates` (`self.TheOnOffer`)))

(event `/Game/Objects/BP_ButtonInterface.SwitchState`
  (params (TheOnOffState :type "/Game/Objects/Misc/E_OnOFfStates Enum" :default "NewEnumerator0"))
  (bind _particlesystem (`self.ParticleSystem`))
  (bind _output_get (set `self.TheOnOffer` TheOnOffState))
  (switch `/Game/Objects/Misc/E_OnOFfStates` _output_get
    (:`NewEnumerator0`
      (`SceneComponent.SetVisibility` _particlesystem true false))
    (:`NewEnumerator1`
      (`SceneComponent.SetVisibility` _particlesystem false false))))

(event `self.Trigger.OnComponentBeginOverlap`
  (params (OverlappedComponent :type "PrimitiveComponent Object Reference") (OtherActor :type "Actor Object Reference") (OtherComp :type "PrimitiveComponent Object Reference") (OtherBodyIndex :type Integer) (bFromSweep :type Boolean) (SweepResult :type "HitResult Structure (by ref)"))
  (cast `/Game/BlueprintCharacters/PhasePlayerCharacter` OtherActor)
  (set `self.HasHitBoxCollision` true))

(event `self.Trigger.OnComponentEndOverlap`
  (params (OverlappedComponent :type "PrimitiveComponent Object Reference") (OtherActor :type "Actor Object Reference") (OtherComp :type "PrimitiveComponent Object Reference") (OtherBodyIndex :type Integer))
  (cast `/Game/BlueprintCharacters/PhasePlayerCharacter` OtherActor)
  (set `self.HasHitBoxCollision` false))

(event `Move`
  (if (`|EnumEquality` (`self.TheOnOffer`) "NewEnumerator0")
    (`/Engine/EditorBlueprintResources/StandardMacros.DoOnce` false :!label _label
      (:`Completed`
        (bind _capsulecomponent (`Character.CapsuleComponent` (stale `self.ReceiveTick` _asphase_player_character)))
        (`KismetSystemLibrary.MoveComponentTo` _capsulecomponent (`SceneComponent.K2_GetComponentLocation` (`self.Arrow`)) (`KismetMathLibrary.Conv_VectorToRotator` (+ (`SceneComponent.GetForwardVector` _capsulecomponent) (`KismetMathLibrary.Conv_RotatorToVector` (`SceneComponent.RelativeRotation` _capsulecomponent)))) true true)
        (`MovementComponent.StopMovementImmediately` (`Character.CharacterMovement` (stale `self.ReceiveTick` _asphase_player_character)))))))

(event `Rest`
  (goto _label :!via `Reset`))

(event `self.ReceiveTick`
  (params (DeltaSeconds :type "Float (single-precision)"))
  (bind _actionbuttonfrompole (`self.ActionButtonfromPole`))
  (`|ExecutionSequence`
    (:`then_0`
      (bind _asphase_player_character (cast `/Game/BlueprintCharacters/PhasePlayerCharacter` (`GameplayStatics.GetPlayerCharacter` 0)))
      (set `self.ActionButtonfromPole` (`/Game/BlueprintCharacters/PhasePlayerCharacter.AxctionButtonActive` _asphase_player_character))
      (if (and _actionbuttonfrompole (`self.HasHitBoxCollision`))
        (`self.Move`)))
    (:`then_1`
      (if (not _actionbuttonfrompole)
        (`self.Rest`)))))

(fn `UserConstructionScript`)