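; BP_NewKeyCard is an interactable key card that the player picks up and carries.
; Interact calls PickUp, which hides the mesh, ignores WorldStatic collision and snaps a component to the supplied target point.
; It then sets KeyCard01 on the PhasePlayerCharacter.
; On GM_ShooterGuy, it becomes the InHand item, joins the InventoryRef list and sets Keycard01Ref.
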(event `PickUp`
  (params (TargetPoint :type "SceneComponent Object Reference") (Actor :type "Actor Object Reference"))
  (bind _keycardmesh (`self.keyCardMesh`))
  (`SceneComponent.SetVisibility` _keycardmesh false false)
  (`PrimitiveComponent.SetCollisionResponseToChannel` _keycardmesh "ECC_WorldStatic" "ECR_Ignore")
  (`self.K2_AttachToComponent` TargetPoint "None" "SnapToTarget" "SnapToTarget" "KeepRelative"))

(fn `Interact`
  (params (TargetPoint :type "SceneComponent Object Reference") (Actor :type "Actor Object Reference"))
  (returns (Val :type Boolean))
  (`self.PickUp` TargetPoint)
  (bind _asphase_player_character (cast `/Game/BlueprintCharacters/PhasePlayerCharacter` Actor))
  (set `/Game/BlueprintCharacters/PhasePlayerCharacter.KeyCard01` true _asphase_player_character)
  (bind _asgm_shooter_guy (cast `/Game/Objects/GamModes/GM_ShooterGuy` (`GameplayStatics.GetGameMode`)))
  (bind _output_get (set `/Game/Objects/GamModes/GM_ShooterGuy.InHand` self _asgm_shooter_guy))
  (`KismetArrayLibrary.Array_Add` (`/Game/Objects/GamModes/GM_ShooterGuy.InventoryRef` _asgm_shooter_guy) _output_get)
  (set `/Game/Objects/GamModes/GM_ShooterGuy.Keycard01Ref` true _asgm_shooter_guy)
  (return false))

(fn `UserConstructionScript`)