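; BP_Button is an interactable button that triggers a linked moving platform.
; Its Interact function calls DoThing and returns false.
; DoThing resolves the owner of the referenced platform, casts it to BP_MovingPlatform and calls MovePlatform, doing nothing if the cast fails.
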(event `DoThing`
  (bind _asbp_moving_platform (cast `/Game/Objects/Blueprints/BP_Interacts/BP_MovingPlatform` (`ActorComponent.GetOwner` (`/Game/Objects/Blueprints/BP_Interacts/BP_MovingPlatform.Platform` (`self.Platform`)))))
  (`/Game/Objects/Blueprints/BP_Interacts/BP_MovingPlatform.MovePlatform` _asbp_moving_platform))

(fn `Interact`
  (params (TargetPoint :type "SceneComponent Object Reference") (Actor :type "Actor Object Reference"))
  (returns (Val :type Boolean))
  (`self.DoThing`)
  (return false))

(fn `UserConstructionScript`
  (`parent.UserConstructionScript`))