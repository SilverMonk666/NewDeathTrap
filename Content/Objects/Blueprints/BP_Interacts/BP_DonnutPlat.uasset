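; BP_DonnutPlat is a platform that moves from its start position toward an EndPoint component when a PhasePlayerCharacter steps on it, and returns when the player leaves.
; BeginPlay caches both world locations and sets the timeline play rate.
; Trigger overlap begin and end play or reverse the MovePlat timeline after separate delays, lerping the platform with sweep enabled.
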(event `self.ReceiveBeginPlay`
  (set `self.Startlocation` (`SceneComponent.K2_GetComponentLocation` (`self.Platform`)))
  (set `self.EndPointLocation` (`SceneComponent.K2_GetComponentLocation` (`self.EndPoint`)))
  (`TimelineComponent.SetPlayRate` (`self.MovePlat`) (`self.PlayRate`)))

(event `self.Trigger.OnComponentBeginOverlap`
  (params (OverlappedComponent :type "PrimitiveComponent Object Reference") (OtherActor :type "Actor Object Reference") (OtherComp :type "PrimitiveComponent Object Reference") (OtherBodyIndex :type Integer) (bFromSweep :type Boolean) (SweepResult :type "HitResult Structure (by ref)"))
  (cast `/Game/BlueprintCharacters/PhasePlayerCharacter` OtherActor)
  (`KismetSystemLibrary.Delay` (`self.DownDelay`))
  (bind (_direction _moveplat) (`Timeline|MovePlat` :!label _label)
    (:`Update`
      (`SceneComponent.K2_SetWorldLocation` (`self.Platform`) (`KismetMathLibrary.VLerp` (`self.Startlocation`) (`self.EndPointLocation`) _moveplat) true false))))

(event `self.Trigger.OnComponentEndOverlap`
  (params (OverlappedComponent :type "PrimitiveComponent Object Reference") (OtherActor :type "Actor Object Reference") (OtherComp :type "PrimitiveComponent Object Reference") (OtherBodyIndex :type Integer))
  (cast `/Game/BlueprintCharacters/PhasePlayerCharacter` OtherActor)
  (`KismetSystemLibrary.Delay` (`self.UpDelay`))
  (goto _label :!via `Reverse`))

(fn `UserConstructionScript`)