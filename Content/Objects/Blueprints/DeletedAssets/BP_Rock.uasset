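; BP_Rock is a moving hazard that slides back and forth and sends characters to their saved checkpoint on contact.
; Tick drives a DoOnce that eases the Gumba component along relative X by Distance over Time, pauses briefly, flips HasMadeIt and resets for the opposite leg.
; Any Character overlapping Trigger calls ResSpawn on BPCCheckPointSave with CheckPointSave.
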(event `self.ReceiveTick`
  (params (DeltaSeconds :type "Float (single-precision)"))
  (bind _gumba (`self.Gumba`))
  (bind (_relativelocation_x _relativelocation_y _relativelocation_z) (`KismetMathLibrary.BreakVector` (`SceneComponent.RelativeLocation` _gumba)))
  (bind (_relativelocation_x_2 _relativelocation_y_2 _relativelocation_z_2) (`KismetMathLibrary.BreakVector` (`SceneComponent.RelativeLocation` _gumba)))
  (`/Engine/EditorBlueprintResources/StandardMacros.DoOnce` false :!label _label
    (:`Completed`
      (if (`self.HasMadeIt`)
        (`KismetSystemLibrary.MoveComponentTo` _gumba (`KismetMathLibrary.MakeVector` (+ _relativelocation_x (`self.Distance`)) _relativelocation_y _relativelocation_z) (`SceneComponent.RelativeRotation` _gumba) true true (`self.Time`))
        (`KismetSystemLibrary.Delay` 0.2)
        (set `self.HasMadeIt` false)
        (goto _label :!via `Reset`)
        (else
          (`KismetSystemLibrary.MoveComponentTo` _gumba (`KismetMathLibrary.MakeVector` (- _relativelocation_x_2 (`self.Distance`)) _relativelocation_y_2 _relativelocation_z_2) (`SceneComponent.RelativeRotation` _gumba) true true (`self.Time`))
          (`KismetSystemLibrary.Delay` 0.2)
          (set `self.HasMadeIt` true)
          (goto _label :!via `Reset`))))))

(event `self.Trigger.OnComponentBeginOverlap`
  (params (OverlappedComponent :type "PrimitiveComponent Object Reference") (OtherActor :type "Actor Object Reference") (OtherComp :type "PrimitiveComponent Object Reference") (OtherBodyIndex :type Integer) (bFromSweep :type Boolean) (SweepResult :type "HitResult Structure (by ref)"))
  (cast `Character` OtherActor)
  (`/Game/Objects/Blueprints/BPC/BPC_CheckPointSave.ResSpawn` (`self.BPC_CheckPointSave`) (`self.CheckPointSave`)))

(fn `UserConstructionScript`)