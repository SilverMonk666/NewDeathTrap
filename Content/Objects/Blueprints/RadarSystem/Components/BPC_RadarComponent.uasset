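; BPC_RadarComponent is an actor component that creates and controls the player's on-screen radar widget.
; Initialization creates the W_Main widget, adds it to the viewport and caches its RadarWidget.
; SetVisibility shows or hides the radar, optionally playing the BlendOut animation forward or reversed, with a flag blocking new changes until the animation ends.
; ToggleVisibility flips the current state through SetVisibility.
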(event `initializeRadar`
  (bind _returnvalue (`|CreateWidget` "/Game/Objects/Blueprints/RadarSystem/Widgets/W_Main.W_Main_C"))
  (bind _output_get (set `self.MainWidgetReference` _returnvalue))
  (set `self.RadarWidgetReference` (`/Game/Objects/Blueprints/RadarSystem/Widgets/W_Main.RadarWidget` _output_get))
  (`UserWidget.AddToViewport` (`self.MainWidgetReference`) 0))

(event `SetVisibility`
  (params (`Visibile?` :type Boolean) (`Animate?` :type Boolean))
  (bind _radarwidgetreference (`self.RadarWidgetReference`))
  (bind _blendout (`/Game/Objects/Blueprints/RadarSystem/Widgets/W_Radar.BlendOut` _radarwidgetreference))
  (bind _blendout_2 (`/Game/Objects/Blueprints/RadarSystem/Widgets/W_Radar.BlendOut` _radarwidgetreference))
  (if (and (!= `Visibile?` (`self.Visible?`)) (`self.CanChangeVisibility?`))
    (set `self.CanChangeVisibility?` false)
    (set `self.Visible?` `Visibile?`)
    (if `Animate?`
      (if (`self.Visible?`)
        (`Widget.SetVisibility` _radarwidgetreference "SelfHitTestInvisible")
        (`UserWidget.PlayAnimation` _radarwidgetreference _blendout 0.0 1 "Reverse" 1.0)
        (`KismetSystemLibrary.Delay` (`WidgetAnimation.GetEndTime` _blendout))
        (set `self.CanChangeVisibility?` true)
        (else
          (`UserWidget.PlayAnimation` _radarwidgetreference _blendout_2 0.0 1 "Forward" 1.0)
          (`KismetSystemLibrary.Delay` (`WidgetAnimation.GetEndTime` _blendout_2))
          (`Widget.SetVisibility` (`self.RadarWidgetReference`) "Hidden")
          (set `self.CanChangeVisibility?` true)))
      (else
        (`Widget.SetVisibility` (`self.RadarWidgetReference`) (select `bool` (`self.Visible?`) :`false` "Hidden" :`true` "SelfHitTestInvisible" :!type "ESlateVisibility Enum"))
        (set `self.CanChangeVisibility?` true)))))

(fn `toggleVisibility`
  (params (`Animate?` :type Boolean :default true))
  (`self.SetVisibility` (not (`self.Visible?`)) `Animate?`)
  (return))